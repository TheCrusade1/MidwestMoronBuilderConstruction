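; Building manager that handles grid-snapped placement previews and timed construction of BP_BuildingMaster actors.
; A fast looping timer moves the preview to the snapped cursor position, with queries for validity, overlap and slope.
; Spawned constructions join a list ticked by a second timer, adding time scaled by GameState's game speed and advancing staged meshes by progress.
; Completion handling is still empty, and worker-unit scaling is only noted as future work.
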(event Custom|SetPreview
  (params (RowName :type Name))
  ;[1 1 1] Set Preview
  (if (Preview|GetIsPreviewing)
    (CallFunction|DestoryPreview))
  (CallFunction|SpawnPreviewBuilding RowName)
  (Preview|SetIsPreviewing true)
  (bind _returnvalue (Utilities|Time|SetTimerbyEvent (EventDispatchers|CreateEvent :!event Custom|TrackCursor) 0.01 true))
  (Variables|Preview|SetPreviewTimerHandle _returnvalue))

(event Custom|SpawnPreviewBuilding
  (params (RowName :type Name))
  ;[1 1 1] Spawn Preview Building
  (Variables|Preview|SetPreviewTransform (Math|Conversions|ToTransform(Vector) (Preview|GetGridSnaps)))
  (bind _returnvalue (Game|SpawnActorfromClass "/Game/Building/Buildings/BP_BuildingMaster.BP_BuildingMaster_C" (Variables|Preview|GetPreviewTransform) "AdjustIfPossibleButAlwaysSpawn" "MultiplyWithRoot" 0 RowName "NewEnumerator0" 0))
  (Utilities|IsValid _returnvalue
    (:Is%20Valid
      (bind _output_get (Variables|References|SetBuildingRef _returnvalue))
      (Default|SetConstructionStatus _output_get "NewEnumerator0"))))

(event Custom|Destory%20Preview
  ;[1 1 1] Destory Preview
  (bind _buildingref (Variables|References|GetBuildingRef)
    (:then
      (Default|DestroyPreview _buildingref)
      (Variables|References|SetBuildingRef 0)
      (Preview|SetIsPreviewing false)
      (Utilities|Time|ClearandInvalidateTimerbyHandle (Variables|Preview|GetPreviewTimerHandle)))
    (:else)))

(event Custom|TrackCursor
  (bind _buildingref (Variables|References|GetBuildingRef))
  ;[1 1 1] Track Cursor
  (Utilities|IsValid _buildingref
    (:Is%20Valid
      (Default|MovePreview _buildingref (Preview|GetGridSnaps)))))

(event Custom|UdateGameSpeed
  (params (GameSpeed :type Float%20%28double-precision%29))
  ;[1 1 1] Update Game Speed
  (bind _output_get (Variables|GameSpeed|SetGameSpeed GameSpeed))
  (Variables|GameSpeed|SetSpeedMultiplier (CallFunction|SetSpeedMultiplier (CallFunction|SetSpeedSetting _output_get))))

(event EventBeginPlay
  (bind _returnvalue (Game|GetGameState))
  (bind _gamestate (Class|BPIGameState|GetGameState(Message) _returnvalue))
  (EventDispatchers|BindEventtoGameSpeedControl _gamestate (EventDispatchers|CreateEvent :!event Custom|UdateGameSpeed))
  (Class|BPIGameTime|UpdateGameSpeed(Message) _returnvalue (Variables|GameSpeed|GetGameSpeed)))

(fn GetIsPreviewing
  (return (Variables|Preview|GetbisPreviewing)))

(fn SetIsPreviewing
  (params (bIsPreviewing :type Boolean))
  (Variables|Preview|SetbisPreviewing bIsPreviewing)
  (return))

(fn GetGridSnaps
  (bind _cursor_position (Variables|Preview|GetCursor%20Position))
  (bind _snapvalues (Variables|Preview|GetSnapValues))
  (bind _snapvalues_2 (Variables|Preview|GetSnapValues))
  (return (Math|Vector|MakeVector (Math|Conversions|ToFloat(Integer) (* (/ (Math|Float|Floor (+ (.x _cursor_position) 5e+01)) _snapvalues) _snapvalues)) (Math|Conversions|ToFloat(Integer) (* (/ (Math|Float|Floor (+ (.y _cursor_position) 5e+01)) _snapvalues_2) _snapvalues_2)) (.z _cursor_position))))

(fn SetCursorPosition
  (params (CursorPosition :type Vector))
  (Variables|Preview|SetCursor%20Position CursorPosition)
  (return))

(fn GetIsPreviewValid
  (bind _buildingref (Variables|References|GetBuildingRef))
  (return (and (Utilities|IsValid _buildingref) (Utilities|Enum|Equal(Enum) (Default|GetConstructionStatus _buildingref) "NewEnumerator0"))))

(fn GetIsPreviewOverlapping
  (return (Default|CheckIsOverlapping (Variables|References|GetBuildingRef))))

(fn GetIsPreviewonSlope
  (return (Default|GetIsonSlope (Variables|References|GetBuildingRef))))

(fn StoreVariables
  (bind _buildingref (Variables|References|GetBuildingRef))
  (Variables|Construction|FromPreview|SetBuildingTransform (Transformation|GetActorTransform _buildingref))
  (Variables|Construction|FromPreview|SetBuildingRowName (Default|GetBuildingRowName _buildingref))
  (return))

(fn SpawnConstruction
  (bind _returnvalue (Game|SpawnActorfromClass "/Game/Building/Buildings/BP_BuildingMaster.BP_BuildingMaster_C" (Variables|Construction|FromPreview|GetBuildingTransform) "Undefined" "MultiplyWithRoot" 0 (Variables|Construction|FromPreview|GetBuildingRowName) "NewEnumerator1" 0))
  (if (!= _returnvalue 0)
    (bind _output_get (LocalVariables|SetBuilding%20Local _returnvalue))
    (Default|SetBuildingStatus _output_get)
    (Construction|AddtoUnconstructionList _output_get)
    (Construction|SetConstructionTimer)))

(fn AddtoUnconstructionList
  (params (NewBuilding :type BP%20Building%20Master%20Object%20Reference))
  (Utilities|IsValid NewBuilding
    (:Is%20Valid
      (Utilities|Array|AddUnique (Variables|Construction|GetListOfUnderConstructionBuilding) NewBuilding))))

(fn SetConstructionTimer
  (if (>= (Utilities|Array|LastIndex (Variables|Construction|GetListOfUnderConstructionBuilding)) 0)
    (if (not (Utilities|Time|IsTimerActivebyHandle (Variables|Construction|GetConstructionTimerHandle)))
      (bind _returnvalue (Utilities|Time|SetTimerbyFunctionName 0 "RunConstructionEvent" (Variables|Construction|Settings|GetBaseConstructionSpeed) true))
      (Variables|Construction|SetConstructionTimerHandle _returnvalue))
    (elif (or (Utilities|Time|IsTimerActivebyHandle (Variables|Construction|GetConstructionTimerHandle)) (Utilities|Time|IsValidTimerHandle (Variables|Construction|GetConstructionTimerHandle)))
      (Utilities|Time|ClearandInvalidateTimerbyHandle (Variables|Construction|GetConstructionTimerHandle)))))

(fn RunConstructionEvent
  ;[1 1 1] In Future, working units > 0
  (if true
    (for _array_element (Variables|Construction|GetListOfUnderConstructionBuilding)
      (LocalVariables|SetBuildingLocal _array_element)
      (if (Utilities|Enum|Equal(Enum) (Default|GetConstructionStatus (LocalVariables|GetBuildingLocal)) "NewEnumerator1")
        (bind _output_get (LocalVariables|SetDeltaConstructionTimeLocal (/ (Variables|Construction|Settings|GetBaseConstructionSpeed) (Variables|GameSpeed|GetSpeedMultiplier))))
        (Default|AddConstructedTime (LocalVariables|GetBuildingLocal) _output_get)
        (switch int (Utilities|Array|Length (Utilities|Struct|BreakFBuildingStruct (Default|GetBuildingData (LocalVariables|GetBuildingLocal))))
          (:1
            _)
          (:2
            (if (and (>= (/ (Default|GetTimeConstructed (LocalVariables|GetBuildingLocal)) (Default|GetConstructionTime (LocalVariables|GetBuildingLocal))) 0.5) (!= (Default|GetBuildingStatus (LocalVariables|GetBuildingLocal)) 1))
              (Default|SetBuildingStatus (LocalVariables|GetBuildingLocal) 1)))
          (:3
            (if (and (and (>= (/ (Default|GetTimeConstructed (LocalVariables|GetBuildingLocal)) (Default|GetConstructionTime (LocalVariables|GetBuildingLocal))) 0.33) (< (/ (Default|GetTimeConstructed (LocalVariables|GetBuildingLocal)) (Default|GetConstructionTime (LocalVariables|GetBuildingLocal))) 0.66)) (!= (Default|GetBuildingStatus (LocalVariables|GetBuildingLocal)) 1))
              (Default|SetBuildingStatus (LocalVariables|GetBuildingLocal) 1))
            (if (and (>= (/ (Default|GetTimeConstructed (LocalVariables|GetBuildingLocal)) (Default|GetConstructionTime (LocalVariables|GetBuildingLocal))) 0.66) (!= (Default|GetBuildingStatus (LocalVariables|GetBuildingLocal)) 2))
              (Default|SetBuildingStatus (LocalVariables|GetBuildingLocal) 2))))
        (if (>= (Default|GetTimeConstructed (LocalVariables|GetBuildingLocal)) (Default|GetConstructionTime (LocalVariables|GetBuildingLocal)))
          _)))))